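; NPC spawn point that spawns waves of random enemies from its SpawnEnemyType list at its own transform.
; On BeginPlay it binds Spawn_Enemy to the player character's SpawnMoreEnemies event.
; Each call spawns EnemySpawned enemies, then sets the next count from the player's wave count times a random wave rate.
; It unbinds when the wave count equals nine, with debug prints along the way.
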(event Custom|Spawn_Enemy
  (bind _spawn_enemy_type (Variables|Default|GetSpawn_Enemy_Type))
  ;[1 1 1] NPC_Spawn_Point
  (for _index (range 0 (- (Variables|Default|GetEnemy_Spawned?) 1))
    (Game|SpawnActorfromClass (Utilities|Array|Get(acopy) _spawn_enemy_type (Math|Random|RandomInteger (Utilities|Array|Length _spawn_enemy_type))) (Transformation|GetActorTransform) "Undefined" "MultiplyWithRoot" 0 0))
  (Math|Integer|IncrementInt (Variables|Default|GetEnemy_Number?)
    (:%20%20
      (bind _asbp_third_person_character (Utilities|Casting|CastToBP_ThirdPersonCharacter (Game|GetPlayerCharacter 0)))
      (Variables|Default|SetEnemy_Spawned? (* (Variables|/Game/ThirdPerson/Blueprints/BP_ThirdPersonCharacter.BP_ThirdPersonCharacter_C|GetPlayer_Bp_Wave_Count _asbp_third_person_character) (Math|Random|RandomIntegerinRange (Variables|/Game/ThirdPerson/Blueprints/BP_ThirdPersonCharacter.BP_ThirdPersonCharacter_C|GetMin_Wave_Rate _asbp_third_person_character) (Variables|/Game/ThirdPerson/Blueprints/BP_ThirdPersonCharacter.BP_ThirdPersonCharacter_C|GetMax_Wave_Rate _asbp_third_person_character))))
      (Development|PrintString (Utilities|String|ToString(Integer) (Math|Random|RandomIntegerinRange (Variables|/Game/ThirdPerson/Blueprints/BP_ThirdPersonCharacter.BP_ThirdPersonCharacter_C|GetMin_Wave_Rate _asbp_third_person_character) (Variables|/Game/ThirdPerson/Blueprints/BP_ThirdPersonCharacter.BP_ThirdPersonCharacter_C|GetMax_Wave_Rate _asbp_third_person_character))) true true "(R=1.000000,G=0.319260,B=0.000000,A=1.000000)")
      (bind _asbp_third_person_character_2 (Utilities|Casting|CastToBP_ThirdPersonCharacter (Game|GetPlayerCharacter 0)))
      (if (== (Variables|/Game/ThirdPerson/Blueprints/BP_ThirdPersonCharacter.BP_ThirdPersonCharacter_C|GetPlayer_Bp_Wave_Count _asbp_third_person_character_2) 9)
        (Development|PrintString "LOOP LOOP ENNND" true true "(R=0.000000,G=1.000000,B=0.045588,A=1.000000)")
        (EventDispatchers|UnbindEventfromSpawnMoreEnemies _asbp_third_person_character_2 (delegate Custom|Spawn_Enemy))
        (else
          (Development|PrintString "wtfffffffff" true true "(R=1.000000,G=0.000000,B=0.991171,A=1.000000)"))))))

(event EventBeginPlay
  ;[1 1 1] NPC_Spawn_Point
  (bind _asbp_third_person_character (Utilities|Casting|CastToBP_ThirdPersonCharacter (Game|GetPlayerCharacter 0)))
  (EventDispatchers|BindEventtoSpawnMoreEnemies _asbp_third_person_character (delegate Custom|Spawn_Enemy)))

(fn ConstructionScript)