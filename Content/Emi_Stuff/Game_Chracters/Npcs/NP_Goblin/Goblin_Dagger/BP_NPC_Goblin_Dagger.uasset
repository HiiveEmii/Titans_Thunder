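; Dagger goblin enemy NPC that registers in the player's TargetsLeft count, chases the player and attempts a melee attack.
; BeginPlay starts a chase and a delayed one-off random move; pawn sensing re-chases, faces and plays a montage, with sight clearing after a retriggerable delay.
; Hit_Box hits and player overlaps damage the goblin itself.
; At zero health it awards score, decrements TargetsLeft, destroys itself and calls CheckTargetsLeft.
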(event OnSeePawn(PawnSensing)
  (params (Pawn :type Pawn%20Object%20Reference))
  ;[1 1 1] Pawn_See?
  (Variables|Default|SetCan_Attack_Player? true)
  (bind _asbp_third_person_character (Utilities|Casting|CastToBP_ThirdPersonCharacter (Game|GetPlayerCharacter 0)))
  (Utilities|FlowControl|Sequence
    (:then_0
      (Variables|Default|SetCan_see_Player? true)
      (AI|AIMoveTo self "0, 0, 0" _asbp_third_person_character 1e+02 false
        (:then
          (Utilities|Casting|CastToBP_ThirdPersonCharacter Pawn)
          (Transformation|SetActorRotation self (Math|Rotator|FindRelativeLookatRotation (Math|Conversions|ToTransform(Vector) (Transformation|GetActorLocation)) (Transformation|GetActorLocation Pawn)))
          (if (Variables|Default|GetCan_Attack_Player?)
            (Animation|PlayAnimMontage self 0 1.0 "None")))))
    (:then_1
      (Utilities|FlowControl|RetriggerableDelay 3.0)
      (Variables|Default|SetCan_see_Player? false))))

(event OnComponentHit(Hit_Box)
  (params (HitComponent :type Primitive%20Component%20Object%20Reference) (OtherActor :type Actor%20Object%20Reference) (OtherComp :type Primitive%20Component%20Object%20Reference) (NormalImpulse :type Vector :default "0, 0, 0") (Hit :type Hit%20Result%20Structure%20%28by%20ref%29))
  (Utilities|FlowControl|Sequence
    (:then_0
      (Effects|SpawnEmitteratLocation 0 (Transformation|GetWorldLocation (Variables|Default|GetHit_Box)))
      (Game|Damage|ApplyDamage self 1e+01 0 0))))

(event OnComponentBeginOverlap(Hit_Box)
  (params (OverlappedComponent :type Primitive%20Component%20Object%20Reference) (OtherActor :type Actor%20Object%20Reference) (OtherComp :type Primitive%20Component%20Object%20Reference) (OtherBodyIndex :type Integer) (bFromSweep :type Boolean) (SweepResult :type Hit%20Result%20Structure%20%28by%20ref%29))
  (Utilities|Casting|CastToBP_ThirdPersonCharacter OtherActor)
  (Game|Damage|ApplyDamage self 2e+01 0 0))

(event EventBeginPlay
  ;[1 1 1] Event_Begin
  (Utilities|FlowControl|Sequence
    (:then_0
      (bind _asbp_third_person_character (Utilities|Casting|CastToBP_ThirdPersonCharacter (Game|GetPlayerCharacter 0)))
      (Variables|/Game/ThirdPerson/Blueprints/BP_ThirdPersonCharacter.BP_ThirdPersonCharacter_C|SetTargets_Left _asbp_third_person_character (+ (Variables|/Game/ThirdPerson/Blueprints/BP_ThirdPersonCharacter.BP_ThirdPersonCharacter_C|GetTargets_Left _asbp_third_person_character) 1)))
    (:then_1
      (AI|AIMoveTo (Class|PawnMovementComponent|GetPawnOwner (Variables|Character|GetCharacterMovement)) "0, 0, 0" (Game|GetPlayerCharacter 0) 5e+01 false))
    (:then_2
      (if (not (Variables|Default|GetCan_see_Player?))
        (Utilities|FlowControl|Delay (Math|Random|RandomFloatinRange 1.0 3.0))
        (AI|AIMoveTo self (.RandomLocation (AI|Navigation|GetRandomReachablePointinRadius (Transformation|GetActorLocation) 0.0 0 0)) 0 5.0 false)))))

(event Collision|EventActorBeginOverlap
  (params (OtherActor :type Actor%20Object%20Reference)))

(event EventTick
  (params (DeltaSeconds :type Float%20%28single-precision%29)))

(event Game|Damage|EventAnyDamage
  (params (Damage :type Float%20%28single-precision%29) (DamageType :type Damage%20Type%20Object%20Reference) (InstigatedBy :type Controller%20Object%20Reference) (DamageCauser :type Actor%20Object%20Reference))
  ;[1 1 1] Any_ DMG?
  (Variables|Default|SetNPC_Health (Math|Float|Clamp(Float) (- (Variables|Default|GetNPC_Health) Damage) 0.0 (Variables|Default|GetNPC_Max_Health)))
  (if (== (Variables|Default|GetNPC_Health) 0.0)
    (Utilities|FlowControl|Sequence
      (:then_0
        (bind _asbp_third_person_character (Utilities|Casting|CastToBP_ThirdPersonCharacter (Game|GetPlayerCharacter 0)))
        (Variables|/Game/ThirdPerson/Blueprints/BP_ThirdPersonCharacter.BP_ThirdPersonCharacter_C|SetScore _asbp_third_person_character (+ (Variables|/Game/ThirdPerson/Blueprints/BP_ThirdPersonCharacter.BP_ThirdPersonCharacter_C|GetScore _asbp_third_person_character) 50)))
      (:then_1
        (bind _asbp_third_person_character_2 (Utilities|Casting|CastToBP_ThirdPersonCharacter (Game|GetPlayerCharacter 0)))
        (Variables|/Game/ThirdPerson/Blueprints/BP_ThirdPersonCharacter.BP_ThirdPersonCharacter_C|SetTargets_Left _asbp_third_person_character_2 (- (Variables|/Game/ThirdPerson/Blueprints/BP_ThirdPersonCharacter.BP_ThirdPersonCharacter_C|GetTargets_Left _asbp_third_person_character_2) 1)))
      (:then_2
        (Actor|DestroyActor))
      (:then_3
        (bind _asbp_third_person_character_3 (Utilities|Casting|CastToBP_ThirdPersonCharacter (Game|Player|GetPlayerPawn 0)))
        (Default|CheckTargetsLeft _asbp_third_person_character_3)))
    (else
      (Development|PrintString (Utilities|String|ToString(Float) (Variables|Default|GetNPC_Health))))))

(fn ConstructionScript)