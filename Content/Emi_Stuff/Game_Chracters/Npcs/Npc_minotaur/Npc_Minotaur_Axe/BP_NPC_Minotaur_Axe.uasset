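; Axe-wielding minotaur enemy NPC that chases the player and counts toward the player's TargetsLeft.
; Pawn sensing rolls random numbers to choose between a melee attack and a delayed spell attack that hides the axe, both reached through AIMoveTo.
; Montage notifies trigger sphere-overlap damage, drawn with debug spheres.
; Damage plays a hit reaction; death awards score and XP, decrements TargetsLeft and destroys the actor.
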(event OnSeePawn(PawnSensing)
  (params (Pawn :type Pawn%20Object%20Reference))
  (bind _returnvalue (Transformation|GetActorLocation))
  (bind _returnvalue_2 (Transformation|GetActorLocation Pawn))
  (bind _returnvalue_3 (Math|Conversions|ToTransform(Vector) _returnvalue))
  (bind _returnvalue_4 (Math|Rotator|FindRelativeLookatRotation _returnvalue_3 _returnvalue_2))
  ;[1 1 1] Pawn_See?
  (Variables|Default|SetCan_See_Random_No (Math|Random|RandomIntegerinRange 1 100) :!label _label)
  (if (>= (Variables|Default|GetCan_See_Random_No) 50) :!label _label_2
    (Variables|Default|SetCan_see_Player? true)
    (else
      (Variables|Default|SetCan_see_Player? false)))
  (if (Variables|Default|GetCan_see_Player?)
    (Transformation|SetActorRotation self (Math|Rotator|MakeRotator (.roll _returnvalue_4) 0.0 (.yaw _returnvalue_4)))
    (Variables|Default|SetRanged_Or_Close_No (Math|Random|RandomIntegerinRange 1 100) :!label _label_3)
    (if (>= (Variables|Default|GetRanged_Or_Close_No) 80)
      (Variables|Default|SetCan_see_Player? false)
      (Variables|Default|SetCan_Attack_Player? true)
      (if (Variables|Default|GetCan_Attack_Player?)
        (AI|AIMoveTo (Class|PawnMovementComponent|GetPawnOwner (Variables|Character|GetCharacterMovement)) "0, 0, 0" (Game|GetPlayerCharacter 0) 1e+02 true
          (:OnSuccess
            (Pawn|Components|CharacterMovement|DisableMovement (Variables|Character|GetCharacterMovement))
            (Utilities|FlowControl|Delay 2.0)
            (CallFunction|SpellAttackMinotaur self)
            (Variables|Default|SetCan_see_Player? false)
            (Variables|Default|SetCan_Attack_Player? false)
            (goto _label_3)))
        (else
          (goto _label_3)))
      (else
        (Variables|Default|SetCan_Attack_Player? true :!label _label_4)
        (Variables|Default|SetCan_see_Player? false)
        (if (Variables|Default|GetCan_Attack_Player?)
          (AI|AIMoveTo (Class|PawnMovementComponent|GetPawnOwner (Variables|Character|GetCharacterMovement)) "0, 0, 0" (Game|GetPlayerCharacter 0) 2e+01 true
            (:OnSuccess
              (CallFunction|BasicAttackMinotuar self)
              (Variables|Default|SetCan_see_Player? false)
              (Variables|Default|SetCan_Attack_Player? false)
              (goto _label_4)))
          (else
            (goto _label_3)))))
    (else
      (Utilities|FlowControl|DoOnce false
        (:Completed
          (Variables|Default|SetTest_Random_No (Math|Random|RandomIntegerinRange 1 100))
          (if (>= 0 50)
            (Pawn|Components|CharacterMovement|DisableMovement (Variables|Character|GetCharacterMovement))
            (Utilities|FlowControl|Delay 1.0)
            (CallFunction|SpellAttackMinotaur self)
            (Variables|Default|SetCan_see_Player? false)
            (Variables|Default|SetCan_Attack_Player? false)
            (goto _label)
            (else
              (goto _label_2))))))))

(event Custom|Spell_Attack_Minotaur
  (bind _spell_attack_animations_minotaur (Variables|Default|GetSpell_Attack_Animations_Minotaur))
  ;[1 1 1] Basic_Attack_Custom_Event
  (Utilities|FlowControl|DoOnce false :!label _label
    (:Completed
      (Pawn|Components|CharacterMovement|DisableMovement (Variables|Character|GetCharacterMovement))
      (Rendering|SetVisibility (Variables|Default|GetAxe_Weapon) false false)
      (Animation|Montage|PlayMontage (Variables|Character|GetMesh) (Utilities|Array|Get(acopy) _spell_attack_animations_minotaur (Math|Random|RandomInteger (Utilities|Array|Length _spell_attack_animations_minotaur)))
        (:OnCompleted
          (Audio|PlaySound2D 0 1.0 1.0 0.0 0 0)
          (Rendering|SetVisibility (Variables|Default|GetAxe_Weapon) true false)
          (Pawn|Components|CharacterMovement|SetMovementMode (Variables|Character|GetCharacterMovement) "MOVE_Walking" 0)
          (goto _label Reset))
        (:OnNotifyBegin
          (CallFunction|DoDmgMinotaur self))))))

(event Custom|Do_Dmg_Minotaur
  (bind _minotaur_attack_radius (Variables|Default|GetMinotaur_Attack_Radius))
  (bind _returnvalue (Transformation|GetWorldLocation _minotaur_attack_radius))
  ;[1 1 1] Do_DMG
  (bind _outactors (Collision|SphereOverlapActors _returnvalue (Variables|Default|GetAttack_Range) (Utilities|Array|MakeArray "ObjectTypeQuery3") "/Script/Engine.Actor" (Utilities|Array|MakeArray self)))
  (Rendering|Debug|DrawDebugSphere _returnvalue (Variables|Default|GetAttack_Range) 12 "(R=1.000000,G=0.000000,B=0.030305,A=1.000000)" 2.0 1.0)
  (for _array_element _outactors
    (Game|Damage|ApplyDamage _array_element (Variables|Default|GetMinotaur_Dmg) (Pawn|GetController) self "/Script/Engine.DamageType")))

(event Custom|Basic_Attack_Minotuar
  (bind _attack_animations_minotaur (Variables|Default|GetAttack_Animations_Minotaur))
  ;[1 1 1] Basic_Attack_Custom_Event
  (Utilities|FlowControl|DoOnce false :!label _label
    (:Completed
      (Pawn|Components|CharacterMovement|DisableMovement (Variables|Character|GetCharacterMovement))
      (Animation|Montage|PlayMontage (Variables|Character|GetMesh) (Utilities|Array|Get(acopy) _attack_animations_minotaur (Math|Random|RandomInteger (Utilities|Array|Length _attack_animations_minotaur))) 1.5
        (:OnCompleted
          (Audio|PlaySound2D 0 1.0 1.0 0.0 0 0)
          (Pawn|Components|CharacterMovement|SetMovementMode (Variables|Character|GetCharacterMovement) "MOVE_Walking" 0)
          (goto _label Reset))
        (:OnNotifyBegin
          (CallFunction|DoDmgMinotaur self))))))

(event Custom|Hit_Reaction_Minotaur
  ;[1 1 1] Hit_Reaction
  (Pawn|Components|CharacterMovement|DisableMovement (Variables|Character|GetCharacterMovement))
  (Components|Animation|PlayAnimation (Variables|Character|GetMesh) "/Game/Emi_Stuff/Game_Chracters/NPCs/Npc_minotaur/Npc_Minotaur_Axe/Animation_Minotaur_Hit_Reaction_Anim_mixamo_com.Animation_Minotaur_Hit_Reaction_Anim_mixamo_com" false)
  (Audio|PlaySound2D 0 1.0 1.0 0.0 0 0)
  (Utilities|FlowControl|Delay 2.0)
  (Pawn|Components|CharacterMovement|SetMovementMode (Variables|Character|GetCharacterMovement) "MOVE_Walking" 0))

(event EventBeginPlay
  ;[1 1 1] Event_Begin
  (Utilities|FlowControl|Sequence
    (:then_0
      (bind _asbp_third_person_character (Utilities|Casting|CastToBP_ThirdPersonCharacter (Game|GetPlayerCharacter 0)))
      (Variables|/Game/ThirdPerson/Blueprints/BP_ThirdPersonCharacter.BP_ThirdPersonCharacter_C|SetTargets_Left _asbp_third_person_character (+ (Variables|/Game/ThirdPerson/Blueprints/BP_ThirdPersonCharacter.BP_ThirdPersonCharacter_C|GetTargets_Left _asbp_third_person_character) 1)))
    (:then_1
      (AI|AIMoveTo (Class|PawnMovementComponent|GetPawnOwner (Variables|Character|GetCharacterMovement)) "0, 0, 0" (Game|GetPlayerCharacter 0) 5e+01 false))
    (:then_2
      (bind _asbp_npc_minotaur_axe (Utilities|Casting|CastToBP_NPC_Minotaur_Axe (Game|GetPlayerCharacter 0)))
      (Variables|BP_NPC_Minotaur_Axe_C|Set%20NP_%20Minotaur_Axe_Ref _asbp_npc_minotaur_axe 0))))

(event Game|Damage|EventAnyDamage
  (params (Damage :type Float%20%28single-precision%29) (DamageType :type Damage%20Type%20Object%20Reference) (InstigatedBy :type Controller%20Object%20Reference) (DamageCauser :type Actor%20Object%20Reference))
  ;[1 1 1] Any_ DMG?
  (CallFunction|HitReactionMinotaur)
  (Variables|Default|SetNPC_Health (Math|Float|Clamp(Float) (- (Variables|Default|GetNPC_Health) Damage) 0.0 (Variables|Default|GetNPC_Max_Health)))
  (if (== (Variables|Default|GetNPC_Health) 0.0)
    (Utilities|FlowControl|Sequence
      (:then_0
        (Utilities|FlowControl|DoOnce false
          (:Completed
            (bind _asbp_third_person_character (Utilities|Casting|CastToBP_ThirdPersonCharacter (Game|GetPlayerCharacter 0)))
            (Variables|/Game/ThirdPerson/Blueprints/BP_ThirdPersonCharacter.BP_ThirdPersonCharacter_C|SetScore _asbp_third_person_character (+ (Variables|/Game/ThirdPerson/Blueprints/BP_ThirdPersonCharacter.BP_ThirdPersonCharacter_C|GetScore _asbp_third_person_character) 50)))))
      (:then_1
        (Utilities|FlowControl|DoOnce false
          (:Completed
            (bind _asbp_third_person_character_2 (Utilities|Casting|CastToBP_ThirdPersonCharacter (Game|GetPlayerCharacter 0)))
            (Variables|/Game/ThirdPerson/Blueprints/BP_ThirdPersonCharacter.BP_ThirdPersonCharacter_C|SetTargets_Left _asbp_third_person_character_2 (- (Variables|/Game/ThirdPerson/Blueprints/BP_ThirdPersonCharacter.BP_ThirdPersonCharacter_C|GetTargets_Left _asbp_third_person_character_2) 1))
            (bind _asbp_third_person_character_3 (Utilities|Casting|CastToBP_ThirdPersonCharacter (Game|GetPlayerCharacter 0))))))
      (:then_2
        (Audio|PlaySound2D 0 1.0 1.0 0.0 0 0)
        (Actor|DestroyActor self))
      (:then_3
        (bind _asbp_third_person_character_4 (Utilities|Casting|CastToBP_ThirdPersonCharacter (Game|GetPlayerCharacter 0)))
        (Default|IncreaseXP _asbp_third_person_character_4 2.0)))
    (else
      (Development|PrintString (Utilities|String|ToString(Float) (Variables|Default|GetNPC_Health)) true true "(R=1.000000,G=0.009597,B=0.000000,A=1.000000)")
      (Development|PrintString "NPC Health" true true "(R=1.000000,G=0.000000,B=0.037429,A=1.000000)"))))

(fn ConstructionScript)