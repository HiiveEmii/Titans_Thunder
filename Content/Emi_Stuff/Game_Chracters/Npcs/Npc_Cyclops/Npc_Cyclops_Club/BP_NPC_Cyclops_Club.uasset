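; Club-wielding cyclops enemy NPC that chases the player and counts toward the player's remaining-target tally.
; On sighting a pawn, random rolls and looping AI moves pick club melee or a fireball spell.
; Montage notifies trigger a sphere overlap damaging "Enemy"-tagged actors, or spawn the fireball.
; Damage plays a hit reaction; death awards score and XP, decrements targets and destroys the actor, leaving ragdoll logic unused.
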(event OnSeePawn(PawnSensing)
  (params (Pawn :type Pawn%20Object%20Reference))
  (bind _returnvalue (Transformation|GetActorLocation))
  (bind _returnvalue_2 (Transformation|GetActorLocation Pawn))
  (bind _returnvalue_3 (Math|Conversions|ToTransform(Vector) _returnvalue))
  (bind _returnvalue_4 (Math|Rotator|FindRelativeLookatRotation _returnvalue_3 _returnvalue_2))
  ;[1 1 1] Pawn_See?
  (Variables|Default|SetCan_See_Random_No (Math|Random|RandomIntegerinRange 1 100) :!label _label)
  (if (>= (Variables|Default|GetCan_See_Random_No) 50) :!label _label_2
    (Variables|Default|SetCan_see_Player? true)
    (else
      (Variables|Default|SetCan_see_Player? false)))
  (if (Variables|Default|GetCan_see_Player?)
    (Transformation|SetActorRotation self (Math|Rotator|MakeRotator (.roll _returnvalue_4) 0.0 (.yaw _returnvalue_4)))
    (Variables|Default|SetRanged_Or_Close_No (Math|Random|RandomIntegerinRange 1 100) :!label _label_3)
    (if (>= (Variables|Default|GetRanged_Or_Close_No) 80)
      (Variables|Default|SetCan_see_Player? false)
      (Variables|Default|SetCan_Attack_Player? true)
      (if (Variables|Default|GetCan_Attack_Player?)
        (AI|AIMoveTo (Class|PawnMovementComponent|GetPawnOwner (Variables|Character|GetCharacterMovement)) "0, 0, 0" (Game|GetPlayerCharacter 0) 1e+02 true
          (:OnSuccess
            (Pawn|Components|CharacterMovement|DisableMovement (Variables|Character|GetCharacterMovement))
            (Utilities|FlowControl|Delay 2.0)
            (CallFunction|SpellAttackCyclops self)
            (Variables|Default|SetCan_see_Player? false)
            (Variables|Default|SetCan_Attack_Player? false)
            (goto _label_3)))
        (else
          (goto _label_3)))
      (else
        (Variables|Default|SetCan_Attack_Player? true :!label _label_4)
        (Variables|Default|SetCan_see_Player? false)
        (if (Variables|Default|GetCan_Attack_Player?)
          (AI|AIMoveTo (Class|PawnMovementComponent|GetPawnOwner (Variables|Character|GetCharacterMovement)) "0, 0, 0" (Game|GetPlayerCharacter 0) 2e+01 true
            (:OnSuccess
              (CallFunction|BasicAttackCyclops self)
              (Variables|Default|SetCan_see_Player? false)
              (Variables|Default|SetCan_Attack_Player? false)
              (goto _label_4)))
          (else
            (goto _label_3)))))
    (else
      (Utilities|FlowControl|DoOnce false
        (:Completed
          (Variables|Default|SetTest_Random_No (Math|Random|RandomIntegerinRange 1 100))
          (if (>= (Variables|Default|GetTest_Random_No) 50)
            (Pawn|Components|CharacterMovement|DisableMovement (Variables|Character|GetCharacterMovement))
            (Utilities|FlowControl|Delay 1.0)
            (CallFunction|SpellAttackCyclops self)
            (goto _label)
            (else
              (goto _label_2))))))))

(event Custom|Spell_Attack_Cyclops
  (bind _spell_attack_animations_cyclops (Variables|Default|GetSpell_Attack_Animations_Cyclops))
  ;[1 1 1] Basic_Attack_Custom_Event
  (Utilities|FlowControl|DoOnce false :!label _label
    (:Completed
      (Pawn|Components|CharacterMovement|DisableMovement (Variables|Character|GetCharacterMovement))
      (Rendering|SetVisibility (Variables|Default|GetClub) false false)
      (Animation|Montage|PlayMontage (Variables|Character|GetMesh) (Utilities|Array|Get(acopy) _spell_attack_animations_cyclops (Math|Random|RandomInteger (Utilities|Array|Length _spell_attack_animations_cyclops))) 1.5
        (:then
          (Audio|PlaySound2D 0 1.0 1.0 0.0 0 0)
          (Rendering|SetVisibility (Variables|Default|GetClub) true false)
          (Utilities|FlowControl|Delay 2.0)
          (Pawn|Components|CharacterMovement|SetMovementMode (Variables|Character|GetCharacterMovement) "MOVE_Walking" 0)
          (goto _label Reset))
        (:OnNotifyBegin
          (Game|SpawnActorfromClass "/Game/Emi_Stuff/VFX/Cyclops/BP_fIREBALL_Cyclops.BP_fIREBALL_Cyclops_C" (Math|Transform|MakeTransform (Transformation|GetWorldLocation (Variables|Default|GetSpell_Cast_Point)) (Transformation|GetActorRotation self) "1.000000,1.000000,1.000000") "Undefined" "MultiplyWithRoot" 0 0))))))

(event Custom|Do_Dmg_Cyclops
  ;[1 1 1] Do_DMG
  (bind _outactors (Collision|SphereOverlapActors (Transformation|GetWorldLocation (Variables|Default|GetClub_Hit_Radius)) (Variables|Default|GetRadius) (Utilities|Array|MakeArray "ObjectTypeQuery3") "/Script/Engine.Actor" (Utilities|Array|MakeArray self (Variables|Default|GetAs%20BP%20NPC%20Minotaur%20Axe) (Variables|Default|GetAs%20BP%20NPC%20Goblin%20Dagger))))
  (for _array_element _outactors
    (if (Actor|ActorHasTag _array_element "Enemy")
      (Game|Damage|ApplyDamage _array_element (Variables|Default|GetCyclops_Base_Damage) (Pawn|GetController) self "/Script/Engine.DamageType"))))

(event Custom|Basic_Attack_Cyclops
  (bind _attack_animations_cyclops (Variables|Default|GetAttack_Animations_Cyclops))
  ;[1 1 1] Basic_Attack_Custom_Event
  (Utilities|FlowControl|DoOnce false :!label _label
    (:Completed
      (Pawn|Components|CharacterMovement|DisableMovement (Variables|Character|GetCharacterMovement))
      (Animation|Montage|PlayMontage (Variables|Character|GetMesh) (Utilities|Array|Get(acopy) _attack_animations_cyclops (Math|Random|RandomInteger (Utilities|Array|Length _attack_animations_cyclops))) 1.5
        (:OnCompleted
          (Audio|PlaySound2D 0 1.0 1.0 0.0 0 0)
          (Pawn|Components|CharacterMovement|SetMovementMode (Variables|Character|GetCharacterMovement) "MOVE_Walking" 0)
          (goto _label Reset))
        (:OnNotifyBegin
          (CallFunction|DoDmgCyclops))))))

(event Custom|Hit_Reaction_Cyclops
  ;[1 1 1] Hit_Reaction
  (Pawn|Components|CharacterMovement|DisableMovement (Variables|Character|GetCharacterMovement))
  (Audio|PlaySound2D 0 1.0 1.0 0.0 0 0)
  (Animation|Montage|PlayMontage (Variables|Character|GetMesh) "/Game/Emi_Stuff/Game_Chracters/NPCs/Npc_Cyclops/Npc_Cyclops_Club/Animation_Cyclops_Hit_Reaction_cyc.Animation_Cyclops_Hit_Reaction_cyc"
    (:OnCompleted
      (Utilities|FlowControl|Delay 0.2)
      (Pawn|Components|CharacterMovement|SetMovementMode (Variables|Character|GetCharacterMovement) "MOVE_Walking" 0))))

(event EventBeginPlay
  ;[1 1 1] Event_Begin
  (Utilities|FlowControl|Sequence
    (:then_0
      (bind _asbp_third_person_character (Utilities|Casting|CastToBP_ThirdPersonCharacter (Game|GetPlayerCharacter 0)))
      (Variables|/Game/ThirdPerson/Blueprints/BP_ThirdPersonCharacter.BP_ThirdPersonCharacter_C|SetTargets_Left _asbp_third_person_character (+ (Variables|/Game/ThirdPerson/Blueprints/BP_ThirdPersonCharacter.BP_ThirdPersonCharacter_C|GetTargets_Left _asbp_third_person_character) 1)))
    (:then_1
      (AI|AIMoveTo (Class|PawnMovementComponent|GetPawnOwner (Variables|Character|GetCharacterMovement)) "0, 0, 0" (Game|GetPlayerCharacter 0) 3e+01 false))))

(event Game|Damage|EventAnyDamage
  (params (Damage :type Float%20%28single-precision%29) (DamageType :type Damage%20Type%20Object%20Reference) (InstigatedBy :type Controller%20Object%20Reference) (DamageCauser :type Actor%20Object%20Reference))
  ;[1 1 1] Any_ DMG?
  (CallFunction|HitReactionCyclops)
  (Variables|Default|SetNPC_Health (Math|Float|Clamp(Float) (- (Variables|Default|GetNPC_Health) Damage) 0.0 (Variables|Default|GetNPC_Max_Health)))
  (if (== (Variables|Default|GetNPC_Health) 0.0)
    (Utilities|FlowControl|Sequence
      (:then_0
        (Utilities|FlowControl|DoOnce false
          (:Completed
            (bind _asbp_third_person_character (Utilities|Casting|CastToBP_ThirdPersonCharacter (Game|GetPlayerCharacter 0)))
            (Variables|/Game/ThirdPerson/Blueprints/BP_ThirdPersonCharacter.BP_ThirdPersonCharacter_C|SetScore _asbp_third_person_character (+ (Variables|/Game/ThirdPerson/Blueprints/BP_ThirdPersonCharacter.BP_ThirdPersonCharacter_C|GetScore _asbp_third_person_character) 50)))))
      (:then_1
        (Utilities|FlowControl|DoOnce false
          (:Completed
            (bind _asbp_third_person_character_2 (Utilities|Casting|CastToBP_ThirdPersonCharacter (Game|GetPlayerCharacter 0)))
            (Variables|/Game/ThirdPerson/Blueprints/BP_ThirdPersonCharacter.BP_ThirdPersonCharacter_C|SetTargets_Left _asbp_third_person_character_2 (- (Variables|/Game/ThirdPerson/Blueprints/BP_ThirdPersonCharacter.BP_ThirdPersonCharacter_C|GetTargets_Left _asbp_third_person_character_2) 1)))))
      (:then_2
        (Audio|PlaySound2D 0 1.0 1.0 0.0 0 0)
        (Actor|DestroyActor self))
      (:then_3
        (bind _asbp_third_person_character_3 (Utilities|Casting|CastToBP_ThirdPersonCharacter (Game|GetPlayerCharacter 0)))
        (Default|IncreaseXP _asbp_third_person_character_3 15.0)))))

(fn ConstructionScript)