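; Ares fireball projectile actor that reacts to what its sphere collider hits and destroys itself after a short lifetime.
; On hitting an Npc-tagged actor, it removes its fire trail, spawns BP_Ares_Explo and calls ApplyDamage with no amount set.
; That branch and other non-player hits share a further spawn call with no class set.
; Player-tagged hits only print a debug string.
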(event OnComponentHit(Sphere)
  (params (HitComponent :type Primitive%20Component%20Object%20Reference) (OtherActor :type Actor%20Object%20Reference) (OtherComp :type Primitive%20Component%20Object%20Reference) (NormalImpulse :type Vector :default "0, 0, 0") (Hit :type Hit%20Result%20Structure%20%28by%20ref%29))
  (if (Actor|ActorHasTag OtherActor "Npc")
    (Components|DestroyComponent (Variables|Default|GetFire_Trail))
    (Game|SpawnActorfromClass "/Game/Emi_Stuff/VFX/Ares/Explosions/BP_Ares_Explo.BP_Ares_Explo_C" (Math|Conversions|ToTransform(Vector) (Transformation|GetWorldLocation (Variables|Default|GetSphere))) "Undefined" "MultiplyWithRoot" 0 0)
    (Game|Damage|ApplyDamage OtherActor 0.0 0 0 "/Script/Engine.DamageType")
    (Game|SpawnActorfromClass "/Game/Emi_Stuff/VFX/Ares/Explosions/BP_Ares_Explo.BP_Ares_Explo_C" (Math|Conversions|ToTransform(Vector) (Transformation|GetWorldLocation (Variables|Default|GetSphere))) "AdjustIfPossibleButAlwaysSpawn" "MultiplyWithRoot" 0 0 :!label _label)
    (elif (Actor|ActorHasTag OtherActor "Player")
      (Development|PrintString "player")
      (else
        (goto _label)))))

(event Collision|EventActorBeginOverlap
  (params (OtherActor :type Actor%20Object%20Reference)))

(event EventTick
  (params (DeltaSeconds :type Float%20%28single-precision%29)))

(event EventBeginPlay
  (Utilities|FlowControl|Sequence
    (:then_0
      (Utilities|FlowControl|Delay 3.0)
      (Utilities|IsValid self
        (:Is%20Valid
          (Actor|DestroyActor self))))))

(fn ConstructionScript)