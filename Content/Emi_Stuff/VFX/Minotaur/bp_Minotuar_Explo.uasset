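; Minotaur explosion actor that acts as a proximity hazard damaging the player.
; On the Sphere's first overlap a DoOnce fires, and if that actor is tagged Player it spawns the minotaur explosion VFX, applies damage and destroys itself after a short delay.
; Because DoOnce runs before the tag check, a non-player overlap uses up the trigger.
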(event OnComponentBeginOverlap(Sphere)
  (params (OverlappedComponent :type Primitive%20Component%20Object%20Reference) (OtherActor :type Actor%20Object%20Reference) (OtherComp :type Primitive%20Component%20Object%20Reference) (OtherBodyIndex :type Integer) (bFromSweep :type Boolean) (SweepResult :type Hit%20Result%20Structure%20%28by%20ref%29))
  (Utilities|FlowControl|DoOnce false
    (:Completed
      (if (Actor|ActorHasTag OtherActor "Player")
        (Niagara|SpawnSystematLocation "/Game/Emi_Stuff/VFX/Minotaur/VFX_Explosion_mINOTAUR.VFX_Explosion_mINOTAUR" (Transformation|GetWorldLocation (Variables|Default|GetSphere)))
        (Game|Damage|ApplyDamage OtherActor 2e+01 0 self "/Script/Engine.DamageType")
        (Utilities|FlowControl|Delay 2.0)
        (Actor|DestroyActor self)))))

(event EventBeginPlay)

(event Collision|EventActorBeginOverlap
  (params (OtherActor :type Actor%20Object%20Reference)))

(event EventTick
  (params (DeltaSeconds :type Float%20%28single-precision%29)))

(fn ConstructionScript)