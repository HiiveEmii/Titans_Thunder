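; Explosion actor for Artemis's Q ability that damages NPCs on contact.
; The first overlap with its Sphere component, guarded by a DoOnce, spawns a leaf explosion effect at the sphere's location.
; If that first actor is tagged NPC, it takes fixed damage and the explosion destroys itself after a short delay.
; Otherwise nothing more happens: later overlaps are ignored and the actor is not destroyed here.
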(event OnComponentBeginOverlap(Sphere)
  (params (OverlappedComponent :type Primitive%20Component%20Object%20Reference) (OtherActor :type Actor%20Object%20Reference) (OtherComp :type Primitive%20Component%20Object%20Reference) (OtherBodyIndex :type Integer) (bFromSweep :type Boolean) (SweepResult :type Hit%20Result%20Structure%20%28by%20ref%29))
  ;[1 1 1] Dmg
  (Utilities|FlowControl|DoOnce false
    (:Completed
      (Niagara|SpawnSystematLocation "/Game/Emi_Stuff/VFX/Artemis/F_Ability/VFX_Explosion_Artemis_Leaf.VFX_Explosion_Artemis_Leaf" (Transformation|GetWorldLocation (Variables|Default|GetSphere)))
      (if (Actor|ActorHasTag OtherActor "NPC")
        (Utilities|FlowControl|DoOnce false
          (:Completed
            (Game|Damage|ApplyDamage OtherActor 1e+01 0 self "/Script/Engine.DamageType")
            (Utilities|FlowControl|Delay 0.2)
            (Actor|DestroyActor self)))))))

(event EventBeginPlay)

(event Collision|EventActorBeginOverlap
  (params (OtherActor :type Actor%20Object%20Reference)))

(event EventTick
  (params (DeltaSeconds :type Float%20%28single-precision%29)))

(fn ConstructionScript)