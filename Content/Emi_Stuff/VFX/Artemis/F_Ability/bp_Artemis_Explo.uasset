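; Explosion actor for Artemis's F ability that spawns a leaf explosion effect and damages an NPC on overlap.
; The first sphere overlap by anything fires a DoOnce and plays the Niagara effect.
; Only if that actor is tagged NPC does it apply damage, read from the player's BP_Ares_2 AresFBaseDmg, then destroy itself after a short delay.
; A non-NPC first overlap uses up the trigger without damage or cleanup.
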(event OnComponentBeginOverlap(Sphere)
  (params (OverlappedComponent :type Primitive%20Component%20Object%20Reference) (OtherActor :type Actor%20Object%20Reference) (OtherComp :type Primitive%20Component%20Object%20Reference) (OtherBodyIndex :type Integer) (bFromSweep :type Boolean) (SweepResult :type Hit%20Result%20Structure%20%28by%20ref%29))
  (Utilities|FlowControl|DoOnce false
    (:Completed
      (Niagara|SpawnSystematLocation "/Game/Emi_Stuff/VFX/Artemis/F_Ability/VFX_Explosion_Artemis_Leaf.VFX_Explosion_Artemis_Leaf" (Transformation|GetWorldLocation (Variables|Default|GetSphere)))
      (if (Actor|ActorHasTag OtherActor "NPC")
        (bind _asbp_ares_2 (Utilities|Casting|CastToBP_Ares_2 (Game|GetPlayerCharacter 0)))
        (Game|Damage|ApplyDamage OtherActor (Variables|/Game/ThirdPerson/Blueprints/BP_Ares_2.BP_Ares_2_C|GetAres_F_Base_dmg _asbp_ares_2) 0 self "/Script/Engine.DamageType")
        (Utilities|FlowControl|Delay 2.0)
        (Actor|DestroyActor self)))))

(event EventBeginPlay)

(event Collision|EventActorBeginOverlap
  (params (OtherActor :type Actor%20Object%20Reference)))

(event EventTick
  (params (DeltaSeconds :type Float%20%28single-precision%29)))

(fn ConstructionScript)