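; BP_fIREBALL_Artemis is a fireball projectile actor for Artemis's F ability.
; The first hit on its Sphere component always destroys it.
; If the hit actor is tagged NPC, it first removes the FireTrail, spawns Bp_Ares_Explo at the impact position and draws a debug sphere there.
; A delay on BeginPlay destroys the fireball after a few seconds if nothing is hit.
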(event OnComponentHit(Sphere)
  (params (HitComponent :type Primitive%20Component%20Object%20Reference) (OtherActor :type Actor%20Object%20Reference) (OtherComp :type Primitive%20Component%20Object%20Reference) (NormalImpulse :type Vector :default "0, 0, 0") (Hit :type Hit%20Result%20Structure%20%28by%20ref%29))
  ;[1 1 1] Fireball_dmg
  (Utilities|FlowControl|DoOnce false
    (:Completed
      (if (Actor|ActorHasTag OtherActor "NPC")
        (Rendering|Debug|DrawDebugSphere (Transformation|GetWorldLocation (Variables|Default|GetSphere)) 1e+02 12 "(R=1.000000,G=0.000000,B=0.030066,A=1.000000)" 1e+01 2.0)
        (Components|DestroyComponent (Variables|Default|GetFire_Trail))
        (Game|SpawnActorfromClass "/Game/Emi_Stuff/VFX/Ares/Explosions/bp_Ares_Explo.bp_Ares_Explo_C" (Math|Conversions|ToTransform(Vector) (Transformation|GetWorldLocation (Variables|Default|GetSphere))) "Undefined" "MultiplyWithRoot" 0 0)
        (Actor|DestroyActor self)
        (else
          (Actor|DestroyActor self))))))

(event Collision|EventActorBeginOverlap
  (params (OtherActor :type Actor%20Object%20Reference)))

(event EventTick
  (params (DeltaSeconds :type Float%20%28single-precision%29)))

(event EventBeginPlay
  ;[1 1 1] EVENT_Begin
  (Utilities|FlowControl|Sequence
    (:then_0
      (Utilities|FlowControl|Delay 5.0)
      (Actor|DestroyActor self))))

(fn ConstructionScript)