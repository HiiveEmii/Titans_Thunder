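; BP_Energy_ball is an energy ball actor that damages foes on impact and destroys itself three seconds after spawning.
; The first sphere collision passes a DoOnce gate; a Foe-tagged actor triggers a debug sphere, trail removal and a Zeus explosion effect.
; It then applies the player Bp_Zeus's base damage to that actor.
; A non-foe Player hit only prints a debug string, and any first hit uses up the gate.
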(event OnComponentHit(Sphere)
  (params (HitComponent :type Primitive%20Component%20Object%20Reference) (OtherActor :type Actor%20Object%20Reference) (OtherComp :type Primitive%20Component%20Object%20Reference) (NormalImpulse :type Vector :default "0, 0, 0") (Hit :type Hit%20Result%20Structure%20%28by%20ref%29))
  ;[1 1 1] Fireball_dmg
  (Utilities|FlowControl|DoOnce false
    (:Completed
      (if (Actor|ActorHasTag OtherActor "Foe")
        (Rendering|Debug|DrawDebugSphere (Transformation|GetWorldLocation (Variables|Default|GetSphere)) 1e+02 12 "(R=1.000000,G=0.000000,B=0.030066,A=1.000000)" 1e+01 2.0)
        (Components|DestroyComponent (Variables|Default|GetFire_Trail))
        (Niagara|SpawnSystematLocation "/Game/Emi_Stuff/VFX/Zeus/Explosion/VFX_Explosion_Zeus.VFX_Explosion_Zeus" (Transformation|GetWorldLocation (Variables|Default|GetSphere)))
        (bind _asbp_zeus (Utilities|Casting|CastToBp_Zeus (Game|GetPlayerCharacter 0)))
        (Game|Damage|ApplyDamage OtherActor (Variables|/Game/ThirdPerson/Blueprints/Bp_Zeus.Bp_Zeus_C|GetF_Base_dmg _asbp_zeus) 0 self "/Script/Engine.DamageType")
        (elif (Actor|ActorHasTag OtherActor "Player")
          (Development|PrintString "player"))))))

(event Collision|EventActorBeginOverlap
  (params (OtherActor :type Actor%20Object%20Reference)))

(event EventTick
  (params (DeltaSeconds :type Float%20%28single-precision%29)))

(event EventBeginPlay
  ;[1 1 1] EVENT_Begin
  (Utilities|FlowControl|Sequence
    (:then_0
      (Utilities|FlowControl|Delay 3.0)
      (Utilities|IsValid self
        (:Is%20Valid
          (Actor|DestroyActor self))))))

(fn ConstructionScript)