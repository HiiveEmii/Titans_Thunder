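; Explosion actor for Zeus's F attack that deals area damage to NPCs.
; The first overlap on its Sphere fires once, gathering pawns within the sphere radius, spawning the Zeus explosion VFX and drawing a debug sphere.
; Each gathered actor tagged NPC takes a small fixed damage hit.
; The actor destroys itself when any overlap with the Sphere ends, with no timed cleanup.
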(event OnComponentEndOverlap(Sphere)
  (params (OverlappedComponent :type Primitive%20Component%20Object%20Reference) (OtherActor :type Actor%20Object%20Reference) (OtherComp :type Primitive%20Component%20Object%20Reference) (OtherBodyIndex :type Integer))
  (Actor|DestroyActor self))

(event OnComponentBeginOverlap(Sphere)
  (params (OverlappedComponent :type Primitive%20Component%20Object%20Reference) (OtherActor :type Actor%20Object%20Reference) (OtherComp :type Primitive%20Component%20Object%20Reference) (OtherBodyIndex :type Integer) (bFromSweep :type Boolean) (SweepResult :type Hit%20Result%20Structure%20%28by%20ref%29))
  (bind _sphere (Variables|Default|GetSphere))
  (bind _sphere_2 (Variables|Default|GetSphere))
  (bind _returnvalue (Components|Sphere|GetScaledSphereRadius _sphere))
  (bind _returnvalue_2 (Transformation|GetWorldLocation _sphere_2))
  (Utilities|FlowControl|DoOnce false
    (:Completed
      (bind _outactors (Collision|SphereOverlapActors _returnvalue_2 _returnvalue (Utilities|Array|MakeArray "ObjectTypeQuery3") "/Script/Engine.Actor" (Utilities|Array|MakeArray self)))
      (Niagara|SpawnSystematLocation "/Game/Emi_Stuff/VFX/Zeus/F_Attack/VFX_Explosion_Zeus.VFX_Explosion_Zeus" (Transformation|GetWorldLocation (Variables|Default|GetSphere)))
      (Rendering|Debug|DrawDebugSphere _returnvalue_2 _returnvalue 12 "(R=1.000000,G=0.000000,B=0.030305,A=1.000000)" 2.0 1.0)
      (for _array_element _outactors
        (if (Actor|ActorHasTag _array_element "NPC")
          (Game|Damage|ApplyDamage _array_element 5.0 0 self "/Script/Engine.DamageType"))))))

(event EventBeginPlay)

(event Collision|EventActorBeginOverlap
  (params (OtherActor :type Actor%20Object%20Reference)))

(event EventTick
  (params (DeltaSeconds :type Float%20%28single-precision%29)))

(fn ConstructionScript)