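; Damage actor for Zeus's E attack, an explosive tornado that hurts NPCs on contact.
; Every overlap on its Sphere spawns the big Zeus explosion effect at the sphere's location, whatever the other actor is.
; A DoOnce limits fixed damage to the first overlapping actor tagged NPC, then the actor destroys itself after a short delay.
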(event OnComponentBeginOverlap(Sphere)
  (params (OverlappedComponent :type Primitive%20Component%20Object%20Reference) (OtherActor :type Actor%20Object%20Reference) (OtherComp :type Primitive%20Component%20Object%20Reference) (OtherBodyIndex :type Integer) (bFromSweep :type Boolean) (SweepResult :type Hit%20Result%20Structure%20%28by%20ref%29))
  ;[1 1 1] Dmg
  (Niagara|SpawnSystematLocation "/Game/Emi_Stuff/VFX/Zeus/Q_Attack/VFX_Explosion_big_Zeus.VFX_Explosion_big_Zeus" (Transformation|GetWorldLocation (Variables|Default|GetSphere)))
  (if (Actor|ActorHasTag OtherActor "NPC")
    (Utilities|FlowControl|DoOnce false
      (:Completed
        (Game|Damage|ApplyDamage OtherActor 1e+01 0 self "/Script/Engine.DamageType")
        (Utilities|FlowControl|Delay 2.0)
        (Actor|DestroyActor self)))))

(fn ConstructionScript)